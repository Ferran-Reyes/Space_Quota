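; Player-controlled spaceship pawn with Enhanced Input for forward and vertical thrust, mouse aim, roll and boost.
; Look input fills a clamped Aim offset that Tick gradually consumes as local axis-angle rotation, with roll applied separately.
; Boost raises FloatingPawnMovement speed and acceleration while held during forward input, draining a charge that recharges only once released.
; The spring arm length eases toward a distance mapped from current speed.
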(event `self.ReceiveBeginPlay`
  (`EnhancedInputSubsystemInterface.AddMappingContext` (pcsubsystem `EnhancedInputLocalPlayerSubsystem` (`GameplayStatics.GetPlayerController` 0)) "/Game/Space_Quota/Input/IMC_Spaceship.IMC_Spaceship" 0 (struct)))

(event `self.ReceiveTick`
  (params (DeltaSeconds :type "Float (single-precision)"))
  (`self.UpdateRotation` DeltaSeconds)
  (`self.UpdateBoost` DeltaSeconds)
  (`self.UpdateCamera` DeltaSeconds))

(event `EnhancedInput|/Game/Space_Quota/Input/IA_MoveForward`
  (params (ActionValue :type "Float (double-precision)") (ElapsedSeconds :type "Float (double-precision)") (TriggeredSeconds :type "Float (double-precision)") (InputAction :type "InputAction Object Reference" :default "/Game/Space_Quota/Input/IA_MoveForward.IA_MoveForward"))
  (:`Triggered`
    (`self.AddMovementInput` (`self.GetActorForwardVector`) ActionValue))
  (:`Started`
    (set `self.IsAccelerating` true))
  (:`Canceled`
    (set `self.IsAccelerating` false :!label _label))
  (:`Completed`
    (goto _label)))

(event `EnhancedInput|/Game/Space_Quota/Input/IA_MoveUp`
  (params (ActionValue :type "Float (double-precision)") (ElapsedSeconds :type "Float (double-precision)") (TriggeredSeconds :type "Float (double-precision)") (InputAction :type "InputAction Object Reference" :default "/Game/Space_Quota/Input/IA_MoveUp.IA_MoveUp"))
  (:`Triggered`
    (`self.AddMovementInput` (`self.GetActorUpVector`) ActionValue)))

(event `EnhancedInput|/Game/Space_Quota/Input/IA_Look`
  (params (ActionValue :type "Vector2D Structure") (ElapsedSeconds :type "Float (double-precision)") (TriggeredSeconds :type "Float (double-precision)") (InputAction :type "InputAction Object Reference" :default "/Game/Space_Quota/Input/IA_Look.IA_Look"))
  (:`Triggered`
    (set `self.Aim` (`KismetMathLibrary.ClampAxes2D` (+ (`self.Aim`) (* ActionValue (`self.MouseSensibility`))) (* (`self.MaxAimAngle`) -1.0) (`self.MaxAimAngle`)))))

(event `EnhancedInput|/Game/Space_Quota/Input/IA_Roll`
  (params (ActionValue :type "Float (double-precision)") (ElapsedSeconds :type "Float (double-precision)") (TriggeredSeconds :type "Float (double-precision)") (InputAction :type "InputAction Object Reference" :default "/Game/Space_Quota/Input/IA_Roll.IA_Roll"))
  (:`Triggered`
    (set `self.RollInput` ActionValue))
  (:`Completed`
    (set `self.RollInput` ActionValue)))

(event `EnhancedInput|/Game/Space_Quota/Input/IA_Boost`
  (params (ActionValue :type Boolean) (ElapsedSeconds :type "Float (double-precision)") (TriggeredSeconds :type "Float (double-precision)") (InputAction :type "InputAction Object Reference" :default "/Game/Space_Quota/Input/IA_Boost.IA_Boost"))
  (:`Started`
    (set `self.BoostHeld` true))
  (:`Canceled`
    (set `self.BoostHeld` false :!label _label_2))
  (:`Completed`
    (goto _label_2)))

(fn `UpdateBoost`
  (params (DeltaTime :type "Float (double-precision)"))
  (bind _floatingpawnmovement (`self.FloatingPawnMovement`))
  (bind _floatingpawnmovement_2 (`self.FloatingPawnMovement`))
  (bind _output_get (set `self.IsBoosting` (and (`self.BoostHeld`) (`self.IsAccelerating`) (> (`self.BoostCharge`) 0.0))))
  (if _output_get
    (set `FloatingPawnMovement.MaxSpeed` (`self.BoostMaxSpeed`) _floatingpawnmovement_2)
    (set `FloatingPawnMovement.Acceleration` (`self.BoostAcceleration`) _floatingpawnmovement_2)
    (set `self.BoostCharge` (`KismetMathLibrary.FClamp` (- (`self.BoostCharge`) DeltaTime) 0.0 (`self.MaxBoostCharge`)))
    (else
      (set `FloatingPawnMovement.MaxSpeed` (`self.NormalMaxSpeed`) _floatingpawnmovement)
      (set `FloatingPawnMovement.Acceleration` (`self.NormalAcceleration`) _floatingpawnmovement)
      (if (not (`self.BoostHeld`))
        (set `self.BoostCharge` (`KismetMathLibrary.FClamp` (+ (* (`self.BoostRechargeRate`) DeltaTime) (`self.BoostCharge`)) 0.0 (`self.MaxBoostCharge`)))))))

(fn `UpdateCamera`
  (params (DeltaTime :type "Float (double-precision)"))
  (set `SpringArmComponent.TargetArmLength` (`KismetMathLibrary.FInterpTo` (`SpringArmComponent.TargetArmLength` (`self.SpringArm`)) (`KismetMathLibrary.MapRangeClamped` (`KismetMathLibrary.VSize` (`self.GetVelocity`)) 0.0 (`self.CameraMaxSpeed`) (`self.BaseCameraDistance`) (`self.MaxCameraDistance`)) DeltaTime (`self.CameraResponse`)) (`self.SpringArm`)))

(fn `UpdateRotation`
  (params (DeltaTime :type "Float (double-precision)"))
  (bind _returnvalue (* (`self.Aim`) (`KismetMathLibrary.FClamp` (* (`self.RotationResponse`) DeltaTime))))
  (bind (_x _y) (`KismetMathLibrary.BreakVector2D` _returnvalue))
  (bind _returnvalue_2 (`KismetMathLibrary.MakeVector` 0.0 (* _y -1.0) _x))
  (`self.K2_AddActorLocalRotation` (`KismetMathLibrary.RotatorFromAxisAndAngle` (`KismetMathLibrary.Normal` _returnvalue_2) (`KismetMathLibrary.VSize` _returnvalue_2)))
  (`self.K2_AddActorLocalRotation` (`KismetMathLibrary.MakeRotator` (* (* (`self.RollInput`) (`self.RollSpeed`)) DeltaTime)))
  (set `self.Aim` (- (`self.Aim`) _returnvalue)))

(fn `UserConstructionScript`)